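; AC_Switcher is an actor component that shifts its owner onto the player's Y plane for 2D view and back afterwards.
; It binds to GM_Main's view-switch event and restores the Y saved at BeginPlay when 2D view ends.
; A bounds-sized sphere trace checks the path to the player's Y; if blocked, Tick retries until clear, then moves the owner and disables itself.
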(event Custom|SwitchView
  (params (is2DView :type Boolean) (Player :type BP%20Player%20Object%20Reference))
  (bind _returnvalue (Components|GetOwner))
  (bind _returnvalue_2 (Components|GetOwner))
  (bind _returnvalue_3 (Transformation|GetActorLocation _returnvalue_2))
  (bind _returnvalue_4 (Transformation|GetActorLocation _returnvalue))
  (if is2DView
    (Variables|Default|SetPlayerYLocation (.y (Transformation|GetActorLocation Player)))
    (bind _returnvalue_5 (CallFunction|CheckLinetrace))
    (if _returnvalue_5
      (Components|Tick|SetComponentTickEnabled true)
      (else
        (Transformation|SetActorLocation (Components|GetOwner) (Math|Vector|MakeVector (.x _returnvalue_4) (Variables|Default|GetPlayerYLocation) (.z _returnvalue_4)) false false)))
    (else
      (Transformation|SetActorLocation (Components|GetOwner) (Math|Vector|MakeVector (.x _returnvalue_3) (Variables|Default|GetOriginalYLocation) (.z _returnvalue_3)) false false))))

(event EventTick
  (params (DeltaSeconds :type Float%20%28single-precision%29))
  (bind _returnvalue (Components|GetOwner))
  (bind _returnvalue_2 (Transformation|GetActorLocation _returnvalue))
  (bind _returnvalue_3 (CallFunction|CheckLinetrace))
  (if (not _returnvalue_3)
    (Transformation|SetActorLocation (Components|GetOwner) (Math|Vector|MakeVector (.x _returnvalue_2) (Variables|Default|GetPlayerYLocation) (.z _returnvalue_2)) false false)
    (Components|Tick|SetComponentTickEnabled false)))

(event EventBeginPlay
  (bind _asgm_main (Utilities|Casting|CastToGM_Main (Game|GetGameMode)))
  (EventDispatchers|BindEventtoViewHadBeenSwitched _asgm_main (delegate Custom|SwitchView))
  (Variables|Default|SetOriginalYLocation (.y (Transformation|GetActorLocation (Components|GetOwner)))))

(fn CheckLinetrace
  (bind _returnvalue (Components|GetOwner))
  (bind (_origin _boxextent) (Collision|GetActorBounds _returnvalue false false))
  (bind (_x _y _z) (Math|Vector|BreakVector _origin))
  (bind _returnvalue_2 (Collision|SphereTraceByChannel _origin (Math|Vector|MakeVector _x (Variables|Default|GetPlayerYLocation) _z) (- (Math|Float|Max(Float) (.x _boxextent) (.z _boxextent)) 1e+01) "TraceTypeQuery4" false 0 "ForDuration"))
  (return _returnvalue_2))