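; BP_NonMoveable is a static mesh actor that changes its visibility and collision when the game switches between 2D and 3D views.
; It binds to GM_Main's view-switch event on BeginPlay.
; In 2D, a debug-drawn box trace around its padded bounds keeps collision on a hit, with visibility gated by DefinitiveInvisible; a miss disables both.
; Leaving 2D always restores both, regardless of that flag.
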(event Custom|SwitchVisibility
  (params (is2DView :type Boolean) (Player :type BP%20Player%20Object%20Reference))
  (bind (_origin _boxextent) (Collision|GetActorBounds false false))
  (bind _staticmesh (Variables|Default|GetStaticMesh))
  (if is2DView
    (bind _returnvalue (Collision|BoxTraceByChannel _origin _origin (+ _boxextent 1e+02) "0, 0, 0" "TraceTypeQuery4" false 0 "ForDuration" true "(R=1.000000,G=0.000000,B=0.000000,A=1.000000)" "(R=0.000000,G=1.000000,B=0.000000,A=1.000000)" 2e+01))
    (Collision|SetCollisionEnabled (Variables|Default|GetStaticMesh) (select _returnvalue "QueryAndPhysics" "NoCollision"))
    (Rendering|SetVisibility (Variables|Default|GetStaticMesh) (select _returnvalue (not (Variables|Default|GetdefinitiveInvisible)) false) false)
    (else
      (Collision|SetCollisionEnabled _staticmesh "QueryAndPhysics")
      (Rendering|SetVisibility _staticmesh true false))))

(event EventBeginPlay
  (bind _asgm_main (Utilities|Casting|CastToGM_Main (Game|GetGameMode)))
  (EventDispatchers|BindEventtoViewHadBeenSwitched _asgm_main (delegate Custom|SwitchVisibility)))

(fn ConstructionScript)