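; BP_Button is a pressure button that activates a linked actor while a player or pushable object is inside its box trigger.
; Overlap begin and end events on the Box accept only BP_Player or BP_Pushable actors and raise or lower an Index counter of occupants.
; Each valid entry calls Activate(true) on LinkedActor, and Activate(false) fires only when the count returns to zero.
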(event OnComponentBeginOverlap(Box)
  (params (OverlappedComponent :type Primitive%20Component%20Object%20Reference) (OtherActor :type Actor%20Object%20Reference) (OtherComp :type Primitive%20Component%20Object%20Reference) (OtherBodyIndex :type Integer) (bFromSweep :type Boolean) (SweepResult :type Hit%20Result%20Structure%20%28by%20ref%29))
  (Variables|Default|GetLinkedActor
    (:then
      (Utilities|Casting|CastToBP_Player OtherActor
        (:then
          (Math|Integer|IncrementInt (Variables|Default|GetIndex)
            (:%20%20
              _)))
        (:CastFailed
          (Utilities|Casting|CastToBP_Pushable OtherActor)
          (Math|Integer|IncrementInt (Variables|Default|GetIndex)
            (:%20%20
              _))))
      (Default|Activate (Variables|Default|GetLinkedActor) true))
    (:else)))

(event OnComponentEndOverlap(Box)
  (params (OverlappedComponent :type Primitive%20Component%20Object%20Reference) (OtherActor :type Actor%20Object%20Reference) (OtherComp :type Primitive%20Component%20Object%20Reference) (OtherBodyIndex :type Integer))
  (Variables|Default|GetLinkedActor
    (:then
      (Utilities|Casting|CastToBP_Player OtherActor
        (:then
          _)
        (:CastFailed
          (Utilities|Casting|CastToBP_Pushable OtherActor)))
      (Math|Integer|DecrementInt (Variables|Default|GetIndex)
        (:%20%20
          (if (== (Variables|Default|GetIndex) 0)
            (Default|Activate (Variables|Default|GetLinkedActor) false)))))
    (:else)))

(fn ConstructionScript)