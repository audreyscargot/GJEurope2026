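; Player character that switches between a 3D third-person view and a 2D side view, notifying GM_Main of each switch.
; In 3D it moves relative to the camera with a pitch-clamped spring arm look; in 2D look is disabled and movement is plane-constrained to one camera axis.
; A forward line trace each tick tracks the interact target, toggles its feedback and receives start/stop interact messages from input.
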(event Custom|ForceRot
  (params (isRotForced :type Boolean))
  (Variables|/Script/Engine.CharacterMovementComponent|SetbOrientRotationToMovement (Variables|Character|GetCharacterMovement) (not isRotForced)))

(event Input|EnhancedActionEvents|EnhancedInputActionIA_Look
  (params (ActionValue :type Vector%202D%20Structure) (ElapsedSeconds :type Float%20%28double-precision%29) (TriggeredSeconds :type Float%20%28double-precision%29) (InputAction :type Input%20Action%20Object%20Reference :default "/Game/Inputs/IA_Look.IA_Look"))
  (if (not (Variables|Default|Getis2DCamera))
    (CallFunction|DoLook (.x ActionValue) (.y ActionValue))))

(event Input|EnhancedActionEvents|EnhancedInputActionIA_Move
  (params (ActionValue :type Vector%202D%20Structure) (ElapsedSeconds :type Float%20%28double-precision%29) (TriggeredSeconds :type Float%20%28double-precision%29) (InputAction :type Input%20Action%20Object%20Reference :default "/Game/Inputs/IA_Move.IA_Move"))
  (if (Variables|Default|Getis2DCamera)
    (CallFunction|DoMove2D (.x ActionValue))
    (else
      (CallFunction|DoMove3D (.x ActionValue) (.y ActionValue)))))

(event Input|EnhancedActionEvents|EnhancedInputActionIA_SwitchCamera
  (params (ActionValue :type Boolean) (ElapsedSeconds :type Float%20%28double-precision%29) (TriggeredSeconds :type Float%20%28double-precision%29) (InputAction :type Input%20Action%20Object%20Reference :default "/Game/Inputs/IA_SwitchCamera.IA_SwitchCamera"))
  (:Started
    (CallFunction|ToggleCamera)))

(event Input|EnhancedActionEvents|EnhancedInputActionIA_Jump
  (params (ActionValue :type Boolean) (ElapsedSeconds :type Float%20%28double-precision%29) (TriggeredSeconds :type Float%20%28double-precision%29) (InputAction :type Input%20Action%20Object%20Reference :default "/Game/Inputs/IA_Jump.IA_Jump"))
  (:Started
    (Character|Jump)))

(event Input|EnhancedActionEvents|EnhancedInputActionIA_Interact
  (params (ActionValue :type Boolean) (ElapsedSeconds :type Float%20%28double-precision%29) (TriggeredSeconds :type Float%20%28double-precision%29) (InputAction :type Input%20Action%20Object%20Reference :default "/Game/Inputs/IA_Interact.IA_Interact"))
  (:Started
    (bind _interacttarget (Variables|Default|GetInteractTarget)
      (:then
        (Class|IInteract|Interact(Message) _interacttarget self))
      (:else)))
  (:Canceled
    (bind _interacttarget_2 (Variables|Default|GetInteractTarget :!label _label)
      (:then
        (Class|IInteract|StopInteract(Message) _interacttarget_2 self))
      (:else)))
  (:Completed
    (goto _label)))

(event EventTick
  (params (DeltaSeconds :type Float%20%28single-precision%29))
  (CallFunction|LaunchFeedback))

(event EventBeginPlay
  (bind _asgm_main (Utilities|Casting|CastToGM_Main (Game|GetGameMode)))
  (Variables|Default|SetAs%20GM%20Main _asgm_main))

(fn ConstructionScript)

(fn DoLook
  (params (X :type Float%20%28single-precision%29) (Y :type Float%20%28single-precision%29))
  (bind _springarm (Variables|Default|GetSpringArm))
  (bind _relativerotation (Variables|/Script/Engine.SceneComponent|GetRelativeRotation _springarm))
  (Transformation|SetRelativeRotation _springarm (Math|Rotator|MakeRotator 0.0 (Math|Float|Clamp(Float) (- (.pitch _relativerotation) Y) -3e+01 1e+01) (+ (.yaw _relativerotation) X)) false false))

(fn DoMove3D
  (params (x :type Float%20%28single-precision%29) (y :type Float%20%28single-precision%29))
  (bind _3dcamera (Variables|Default|Get3DCamera))
  (Pawn|Input|AddMovementInput (Math|Vector|GetForwardVector _3dcamera) y false)
  (Pawn|Input|AddMovementInput (Math|Vector|GetRightVector _3dcamera) x false))

(fn ToggleCamera
  (bind _charactermovement (Variables|Character|GetCharacterMovement))
  (Variables|Default|Setis2DCamera (not (Variables|Default|Getis2DCamera)))
  (Components|Activation|SetActive (Variables|Default|Get3DCamera) (not (Variables|Default|Getis2DCamera)) false)
  (Components|Activation|SetActive (Variables|Default|Get2DCamera) (Variables|Default|Getis2DCamera) false)
  (Default|Switch (Variables|Default|GetAs%20GM%20Main) (Variables|Default|Getis2DCamera) self)
  (Class|MovementComponent|SetPlaneConstraintAxisSetting _charactermovement "Y")
  (Class|MovementComponent|SetPlaneConstraintEnabled _charactermovement (Variables|Default|Getis2DCamera))
  (if (Variables|Default|Getis2DCamera)
    (Transformation|SetActorRotation (Math|Rotator|MakeRotator 0.0 0.0 0.0))))

(fn LaunchFeedback
  (bind _capsulecomponent (Variables|Collision|GetCapsuleComponent))
  (bind _returnvalue (Transformation|GetWorldLocation _capsulecomponent))
  (bind _outhit (Collision|LineTraceByChannel _returnvalue (+ _returnvalue (* (Math|Vector|GetForwardVector _capsulecomponent) 5e+02)) "TraceTypeQuery3" false 0 "None"))
  (if (.bBlockingHit (Collision|BreakHitResult _outhit))
    (if (!= (.HitActor (Collision|BreakHitResult _outhit)) (Variables|Default|GetInteractTarget))
      (Class|IInteract|InteractFeedback(Message) (Variables|Default|GetInteractTarget) false)
      (Class|IInteract|StopInteract(Message) (Variables|Default|GetInteractTarget) self)
      (bind _output_get (Variables|Default|SetInteractTarget (.HitActor (Collision|BreakHitResult _outhit))))
      (Class|IInteract|InteractFeedback(Message) _output_get true))
    (else
      (Class|IInteract|InteractFeedback(Message) (Variables|Default|GetInteractTarget) false)
      (Class|IInteract|StopInteract(Message) (Variables|Default|GetInteractTarget) self)
      (Variables|Default|SetInteractTarget 0))))

(fn DoMove2D
  (params (X :type Float%20%28single-precision%29))
  (Pawn|Input|AddMovementInput (Math|Vector|GetRightVector (Variables|Default|Get2DCamera)) X false))