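; BP_Pushable is an interactible actor that follows the player along the world X axis while being pushed.
; Interact stores the player, calls ForceRot on it, records the actor's X offset in player space and enables Tick.
; Tick sets X to the player's X plus that offset and a small constant, keeping Y and Z.
; StopInteract releases ForceRot, disables Tick and clears the player's InteractTarget.
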(event EventInteract
  (params (Player :type BP%20Player%20Object%20Reference))
  (bind _output_get (Variables|Default|SetPlayer Player))
  (Default|ForceRot _output_get true)
  (Variables|Default|SetDistanceX (.x (Math|Transform|InverseTransformLocation (Transformation|GetActorTransform (Variables|Default|GetPlayer)) (Transformation|GetActorLocation))))
  (Actor|Tick|SetActorTickEnabled true))

(event EventTick
  (params (DeltaSeconds :type Float%20%28single-precision%29))
  (bind _returnvalue (Transformation|GetActorLocation))
  (Transformation|SetActorLocation (Math|Vector|MakeVector (+ (.x (Transformation|GetActorLocation (Variables|Default|GetPlayer))) (Variables|Default|GetDistanceX) 1e+01) (.y _returnvalue) (.z _returnvalue)) false false))

(event EventStopInteract
  (params (Player :type BP%20Player%20Object%20Reference))
  (Default|ForceRot Player false)
  (Actor|Tick|SetActorTickEnabled false)
  (Variables|/Game/Blueprints/BP_Player.BP_Player_C|SetInteractTarget Player 0))

(fn ConstructionScript
  (|CallParentFunction))