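; BP_Door is an activatable door that swings open or slams shut through its Activate event.
; It stores the mesh's world rotation at BeginPlay, and a timeline lerps from that rotation to a 90-degree offset.
; Activating plays the timeline slowly with a metal opening sound, while deactivating reverses it at a faster rate with a slam sound, swapped onto the same audio component.
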(event EventActivate
  (params (shouldActivate :type Boolean))
  (bind _timeline (Variables|Default|GetTimeline))
  (bind _buttonup_004_cue (Variables|Default|GetbuttonUp-004_Cue))
  (bind _ogrot (Variables|Default|GetOGRot))
  (bind _buttonup_004_cue_2 (Variables|Default|GetbuttonUp-004_Cue))
  (if shouldActivate
    (Components|Timeline|SetPlayRate _timeline 0.5)
    (Audio|Components|Audio|SetSound _buttonup_004_cue_2 "/Game/SD/metalDoorOpen-003_Cue.metalDoorOpen-003_Cue")
    (Audio|Components|Audio|Play _buttonup_004_cue_2 0.0)
    (bind _alpha (Timeline|Timeline Play)
      (:Update
        (Transformation|SetWorldRotation (Variables|Default|GetStaticMesh) (Math|Rotator|Lerp(Rotator) _ogrot (Math|Rotator|CombineRotators _ogrot "0.000000,90.000000,0.000000") _alpha) false false)))
    (else
      (Components|Timeline|SetPlayRate _timeline 2.0)
      (Audio|Components|Audio|SetSound _buttonup_004_cue "/Game/SD/doorSlam-003_Cue.doorSlam-003_Cue")
      (Audio|Components|Audio|Play _buttonup_004_cue 0.0)
      (Timeline|Timeline Reverse))))

(event EventBeginPlay
  (Variables|Default|SetOGRot (Transformation|GetWorldRotation (Variables|Default|GetStaticMesh))))

(fn ConstructionScript
  (|CallParentFunction))